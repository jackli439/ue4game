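; BP_Gun is a gun item that lies in the world as an interactable pickup and can be equipped or dropped by a player.
; It starts Dropped with a physics-simulated mesh and an overlap sphere, and offers a "PickUp" prompt attached to the mesh.
; Interaction asks the Player to pick it up; on success SetGunState switches to Equipped, disabling physics and collision and resetting the mesh transform.
; Drop restores the Dropped state.
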(event EventBeginPlay
  (Public|SetGunState "NewEnumerator0"))

(event EventOnInteracted
  (params (Player :type Ue%204ASP%20Character%20Object%20Reference))
  (bind _success (Default|PickUpGun Player self))
  (if _success
    (Public|SetGunState "NewEnumerator1")))

(fn ConstructionScript
  (|CallParentFunction))

(fn GetInteractionText
  (return "PickUp"))

(fn GetInteractionTextAttach
  (return (Variables|Default|GetSkeletalMesh)))

(fn SetGunState
  (params (NewGunState :type EquippedGunState%20Enum :default "NewEnumerator0"))
  (bind _skeletalmesh (Variables|Default|GetSkeletalMesh))
  (bind _output_get (Variables|Default|SetGunState NewGunState))
  (switch Utilities|FlowControl|Switch|SwitchonEquippedGunState _output_get
    (:NewEnumerator0
      (Collision|SetCollisionProfileName (Variables|Default|GetSphere) "OverlapAllDynamic" true :!class /Script/Engine.PrimitiveComponent)
      (Physics|SetSimulatePhysics _skeletalmesh true)
      (Collision|SetCollisionProfileName _skeletalmesh "DroppedGun" true :!class /Script/Engine.PrimitiveComponent))
    (:NewEnumerator1
      (Collision|SetCollisionProfileName (Variables|Default|GetSphere) "NoCollision" true :!class /Script/Engine.PrimitiveComponent)
      (Physics|SetSimulatePhysics (Variables|Default|GetSkeletalMesh) false)
      (Collision|SetCollisionProfileName (Variables|Default|GetSkeletalMesh) "NoCollision" true :!class /Script/Engine.PrimitiveComponent)
      (Transformation|ResetRelativeTransform (Variables|Default|GetSkeletalMesh)))))

(fn Drop
  (Public|SetGunState "NewEnumerator0"))